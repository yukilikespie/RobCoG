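; BP_WaterParticles is an interactable actor that lets the player toggle a particle system, named as a water effect, with the E key.
; Its Trigger component enables input for player controller 0 on any begin overlap and disables it on end overlap, without checking which actor overlapped.
; Each E press prints a debug string, then activates or deactivates the ParticleSystem based on whether it is active.
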(event `Key|E`
  (params (Key :type "Key Structure" :default "AnyKey"))
  (bind _particlesystem (`self.ParticleSystem`))
  (:`Pressed`
    (`KismetSystemLibrary.PrintString` "E pressed biatch")
    (if (`ActorComponent.IsActive` (`self.ParticleSystem`))
      (`ActorComponent.Deactivate` _particlesystem)
      (else
        (`ActorComponent.Activate` _particlesystem false)))))

(event `self.Trigger.OnComponentBeginOverlap`
  (params (OverlappedComponent :type "PrimitiveComponent Object Reference") (OtherActor :type "Actor Object Reference") (OtherComp :type "PrimitiveComponent Object Reference") (OtherBodyIndex :type Integer) (bFromSweep :type Boolean) (SweepResult :type "HitResult Structure (by ref)"))
  (`self.EnableInput` (`GameplayStatics.GetPlayerController` 0)))

(event `self.Trigger.OnComponentEndOverlap`
  (params (OverlappedComponent :type "PrimitiveComponent Object Reference") (OtherActor :type "Actor Object Reference") (OtherComp :type "PrimitiveComponent Object Reference") (OtherBodyIndex :type Integer))
  (`self.DisableInput` (`GameplayStatics.GetPlayerController` 0)))

(fn `UserConstructionScript`)